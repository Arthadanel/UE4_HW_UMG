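; BP_Player is the player-controlled pawn in GeometryCatcher, moving left and right along its right vector.
; The MoveRight axis accumulates movement input scaled by MaxSpeed, and Tick consumes it as a frame-rate-independent, swept local offset while the game is not paused.
; On BeginPlay it caches BP_GameManager, which supplies the Paused flag and receives a Pause call when P is pressed.
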(event EventBeginPlay
  (bind _returnvalue (Actor|GetActorOfClass "/Game/GeometryCatcher/Blueprints/BP_GameManager.BP_GameManager_C"))
  (Variables|Default|SetGameManager _returnvalue))

(event EventTick
  (params (DeltaSeconds :type Float%20%28single-precision%29))
  (if (not (Variables|/Game/GeometryCatcher/Blueprints/BP_GameManager.BP_GameManager_C|GetPaused (Variables|Default|GetGameManager)))
    (bind _returnvalue (Class|Pawn|ConsumeMovementInputVector))
    (Transformation|AddActorLocalOffset (* _returnvalue DeltaSeconds) true false)))

(event Input|AxisEvents|InputAxisMoveRight
  (params (AxisValue :type Float%20%28single-precision%29))
  (Pawn|Input|AddMovementInput (Transformation|GetActorRightVector) (* AxisValue (Variables|Default|GetMaxSpeed)) false))

(event Input|KeyboardEvents|P
  (params (Key :type Key%20Structure :default "None"))
  (:Pressed
    (Default|Pause (Variables|Default|GetGameManager))))

(fn ConstructionScript)