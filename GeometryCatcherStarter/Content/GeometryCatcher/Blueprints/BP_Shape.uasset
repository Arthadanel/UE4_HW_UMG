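; BP_Shape is a falling collectible for the Geometry Catcher game, caught by overlapping the player.
; Each tick it moves straight down at FallSpeed with a swept world offset, unless the GameManager is paused.
; On overlap with BP_Player, it passes its Value to the GameManager's total and individual shape counters, then destroys itself.
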(event EventBeginPlay)

(event Collision|EventActorBeginOverlap
  (params (OtherActor :type Actor%20Object%20Reference))
  (Utilities|Casting|CastToBP_Player OtherActor)
  (Default|IncrementShapesCollected (Variables|Default|GetGameManager) (Variables|Default|GetValue))
  (Default|IncrementIndividualShapesCollected (Variables|Default|GetGameManager) (Variables|Default|GetValue))
  (Actor|DestroyActor))

(event EventTick
  (params (DeltaSeconds :type Float%20%28single-precision%29))
  (if (not (Variables|/Game/GeometryCatcher/Blueprints/BP_GameManager.BP_GameManager_C|GetPaused (Variables|Default|GetGameManager)))
    (Transformation|AddActorWorldOffset (Math|Vector|MakeVector 0.0 0.0 (* (* DeltaSeconds (Variables|Default|GetFallSpeed)) -1.0)) true)))

(fn ConstructionScript)